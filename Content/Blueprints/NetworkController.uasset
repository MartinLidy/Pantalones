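; NetworkController is an actor that automatically hosts or joins a LAN multiplayer session five seconds after play begins.
; When Client is true, it searches for a single session and joins it; otherwise it creates a session with ten public connections.
; Each outcome prints an on-screen status message.
; Nodes for reopening ThirdPersonExampleLevel as a listen server are present but never run.
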(event EventBeginPlay
  (bind _returnvalue (Game|GetPlayerController 0))
  (Utilities|FlowControl|Delay 5.0)
  (if (Variables|Default|GetClient)
    (bind _results (|FindSessions _returnvalue 1 true)
      (:OnSuccess
        (|JoinSession 0 (Utilities|Array|Get(acopy) _results)
          (:OnSuccess
            (Development|PrintString "Session Joined!" true true "(R=0.000000,G=1.000000,B=0.146502,A=1.000000)"))
          (:OnFailure
            (Development|PrintString "Session Join Failed" true true "(R=1.000000,G=0.037799,B=0.000000,A=1.000000)"))))
      (:OnFailure
        (Development|PrintString "Session Search Failed" true true "(R=1.000000,G=0.037799,B=0.000000,A=1.000000)")))
    (else
      (|Session _returnvalue 10 true
        (:OnSuccess
          (Development|PrintString "Session Hosted!" true true "(R=0.000000,G=1.000000,B=0.146502,A=1.000000)"))
        (:OnFailure
          (Development|PrintString "Session Creation Failed" true true "(R=1.000000,G=0.037799,B=0.000000,A=1.000000)"))))))

(event EventActorBeginOverlap
  (params (OtherActor :type Actor%20Object%20Reference)))

(event EventTick
  (params (DeltaSeconds :type Float%20%28single-precision%29)))

(fn ConstructionScript)